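; Interactable door Blueprint that swings open or closed when its linked button is pressed or Interact is called.
; Open angle, speed and locked state come from DoorData settings, and a locked door only prints a message.
; A timeline plays or reverses to lerp the DoorPivot yaw, toggling IsOpen when it finishes.
; OpenSpeed is cached on BeginPlay but never applied to the timeline.
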(event `self.ReceiveBeginPlay`
  (add `/Game/Blueprints/BP_Button.OnPressed` (`self.LinkedButton`) (delegate `/Game/Blueprints/Interfaces/BPI_Interactable.Interact`))
  (bind _openangle (`self.GetOpenAngle`))
  (set `self.Open Angle` _openangle)
  (bind _openspeed (`self.GetOpenSpeed`))
  (set `self.Open Speed` _openspeed))

(event `/Game/Blueprints/Interfaces/BPI_Interactable.Interact`
  (bind _islocked (`self.GetLocked`))
  (if _islocked
    (`KismetSystemLibrary.PrintString` "Door Locked" true true (struct :`R` 1.0 :`B` 0.12123 :`A` 1.0))
    (elif (`self.bIsOpen`)
      (bind (_direction _alpha) (`Timeline|TL_OpenDoor` :!via `Reverse` :!label _label)
        (:`Update`
          (`SceneComponent.K2_SetRelativeRotation` (`self.DoorPivot`) (`KismetMathLibrary.MakeRotator` 0.0 0.0 (`KismetMathLibrary.Lerp` 0.0 (`self.Open Angle`) _alpha)) false false))
        (:`Finished`
          (bind _output_get (set `self.bIsOpen` (not (`self.bIsOpen`))))
          (`KismetSystemLibrary.PrintString` (`KismetStringLibrary.Concat_StrStr` "Door is now " (`KismetStringLibrary.Conv_BoolToString` _output_get)) true true (struct :`R` 1.0 :`G` 0.4799 :`B` 0.625204 :`A` 1.0))))
      (else
        (goto _label)))))

(fn `GetLocked`
  (returns (IsLocked :type Boolean))
  (return (`.Locked_1_77D79F524F1B9938F4D5BC870FB1EF7A` (break `/Game/Data/ST_DoorSettings` (`/Game/Data/DA_DoorSettings.Settings` (`self.DoorData`))))))

(fn `GetOpenAngle`
  (returns (OpenAngle :type "Float (double-precision)"))
  (return (`.OpenAngle_4_2879CD7E437761CA7893ED97672095FA` (break `/Game/Data/ST_DoorSettings` (`/Game/Data/DA_DoorSettings.Settings` (`self.DoorData`))))))

(fn `GetOpenSpeed`
  (returns (OpenSpeed :type "Float (double-precision)"))
  (return (`.OpenSpeed_6_45C5F33B401ABB6A8EE5C8A3A3E020C0` (break `/Game/Data/ST_DoorSettings` (`/Game/Data/DA_DoorSettings.Settings` (`self.DoorData`))))))

(fn `UserConstructionScript`)