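; AI controller for a guard that starts the BT_Guard behavior tree on BeginPlay.
; BeginPlay also starts a looping one-second timer, and an EverySeconds event compares the distance between player character 0 and the controller's owner, rather than its controlled pawn, against DetectionRange.
; The in-range branch is empty, so the distance check has no effect.
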(event `self.ReceiveBeginPlay`
  (`self.RunBehaviorTree` "/Game/Blueprints/AI/BT_Guard.BT_Guard")
  (`KismetSystemLibrary.K2_SetTimerDelegate` :`Time` 1.0 :`bLooping` true :`InitialStartDelay` 1.0))

(event `EverySeconds`
  (if (< (`KismetMathLibrary.Vector_Distance` (`self.K2_GetActorLocation` (`GameplayStatics.GetPlayerCharacter` 0)) (`self.K2_GetActorLocation` (`ActorComponent.GetOwner`))) (`self.DetectionRange`))
    _))

(fn `UserConstructionScript`)