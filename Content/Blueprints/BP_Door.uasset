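; BP_Door is an interactable swinging door, configured through DoorData, that opens and closes on direct interaction or a linked button press.
; Interact checks the lock type and, for key-style locks, the required gameplay tag in the interactor's inventory, printing "Door Locked" on failure.
; A timeline plays or reverses to lerp the pivot's yaw to the configured open angle, toggling the open state when finished.
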(event `self.ReceiveBeginPlay`
  (add `/Game/Blueprints/BP_Button.OnPressed` (`self.LinkedButton`) (delegate `/Game/Blueprints/Interfaces/BPI_Interactable.Interact`)))

(event `/Game/Blueprints/Interfaces/BPI_Interactable.Interact`
  (params (Interactor :type "/Game/Blueprints/BP_ContainmentCharacter Object Reference"))
  (bind _canopen (`self.CanOpenDoor` (`/Game/Blueprints/BP_ContainmentCharacter.BPC_Inventory` Interactor)))
  (if _canopen
    (if (`self.bIsOpen`)
      (bind (_direction _alpha) (`Timeline|TL_OpenDoor` :!via `Reverse` :!label _label)
        (:`Update`
          (bind _openangle (`self.GetOpenAngle`))
          (`SceneComponent.K2_SetRelativeRotation` (`self.DoorPivot`) (`KismetMathLibrary.MakeRotator` 0.0 0.0 (`KismetMathLibrary.Lerp` 0.0 _openangle _alpha)) false false))
        (:`Finished`
          (set `self.bIsOpen` (not (`self.bIsOpen`)))))
      (else
        (goto _label)))
    (else
      (`KismetSystemLibrary.PrintString` "Door Locked" true true (struct :`R` 1.0 :`G` 0.030358 :`B` 0.046116 :`A` 1.0)))))

(fn `CanOpenDoor`
  (params (Inventory :type "/Game/Components/BPC_Inventory Object Reference"))
  (returns (CanOpen :type Boolean))
  (bind (_locktype _requiredtag) (break `/Game/Data/ST_LockSettings` (`.LockSettings_13_77D79F524F1B9938F4D5BC870FB1EF7A` (break `/Game/Data/ST_DoorSettings` (`/Game/Data/DA_DoorSettings.Settings` (`self.DoorData`))))))
  (bind _hastag (`/Game/Components/BPC_Inventory.HasGameplayTag` Inventory _requiredtag))
  (return (or (`|EnumEquality` _locktype "NewEnumerator0") (and (`|EnumEquality` _locktype "NewEnumerator1") _hastag))))

(fn `GetDisplayName`
  (returns (DisplayName :type Text))
  (return "Porte"))

(fn `GetOpenAngle`
  (returns (OpenAngle :type "Float (double-precision)"))
  (return (`.OpenAngle_4_2879CD7E437761CA7893ED97672095FA` (break `/Game/Data/ST_DoorSettings` (`/Game/Data/DA_DoorSettings.Settings` (`self.DoorData`))))))

(fn `GetOpenSpeed`
  (returns (OpenSpeed :type "Float (double-precision)"))
  (return (`.OpenSpeed_6_45C5F33B401ABB6A8EE5C8A3A3E020C0` (break `/Game/Data/ST_DoorSettings` (`/Game/Data/DA_DoorSettings.Settings` (`self.DoorData`))))))

(fn `UserConstructionScript`)