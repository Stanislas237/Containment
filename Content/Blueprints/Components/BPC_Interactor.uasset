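; BPC_Interactor is a component that detects which interactable the player's BP_ContainmentCharacter is looking at.
; Each tick it line-traces on Visibility from the player camera out to InteractionDistance, keeping the hit actor only if it implements BPI_Interactable.
; When the target changes, it sends the display name and show state to the character's HUD update.
; CanInteract exposes whether a target exists, along with that actor.
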(event `self.ReceiveTick`
  (params (DeltaSeconds :type "Float (single-precision)"))
  (`self.ScanInteractable`))

(fn `CanInteract`
  (returns (CanInteract :type Boolean) (ActorInteracted :type "Actor Object Reference"))
  (locals (CameraStart :type "Vector Structure" :default (0.0 0.0 0.0)) (CameraEnd :type "Vector Structure"))
  (bind _currentinteractable (`self.CurrentInteractable`))
  (return (!= null _currentinteractable) _currentinteractable))

(fn `ScanInteractable`
  (locals (CameraStart :type "Vector Structure") (CameraEnd :type "Vector Structure") (Character :type "/Game/Blueprints/BP_ContainmentCharacter Object Reference"))
  (bind _asbp_containment_character (cast `/Game/Blueprints/BP_ContainmentCharacter` (`self.GetOwner`)))
  (bind _output_get (set `local.Character` _asbp_containment_character))
  (bind _playercamera (`/Game/Blueprints/BP_ContainmentCharacter.PlayerCamera` _output_get))
  (bind _output_get_2 (set `local.CameraStart` (`SceneComponent.K2_GetComponentLocation` _playercamera)))
  (set `local.CameraEnd` (+ (* (`self.InteractionDistance`) (`SceneComponent.GetForwardVector` _playercamera)) _output_get_2))
  (bind _outhit (`KismetSystemLibrary.LineTraceSingle` :`Start` (`local.CameraStart`) :`End` (`local.CameraEnd`) :`TraceChannel` "TraceTypeQuery1" :`DrawTime` 0.0))
  (bind (_bblockinghit _binitialoverlap _time _distance _location _impactpoint _normal _impactnormal _physmat _hitactor) (`GameplayStatics.BreakHitResult` _outhit))
  (if (`KismetSystemLibrary.DoesImplementInterface` _hitactor "/Game/Blueprints/Interfaces/BPI_Interactable.BPI_Interactable_C")
    (set `self.CurrentInteractable` _hitactor)
    (else
      (set `self.CurrentInteractable` null)))
  (if (!= (`self.LastInteractable`) (`self.CurrentInteractable`))
    (bind _displayname (message `/Game/Blueprints/Interfaces/BPI_Interactable.GetDisplayName` (`self.CurrentInteractable`)))
    (`/Game/Blueprints/BP_ContainmentCharacter.UpdateHUD` (`local.Character`) (!= null (`self.CurrentInteractable`)) _displayname)
    (set `self.LastInteractable` (`self.CurrentInteractable`))))