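; Actor component that handles line-of-sight interaction for its owning BP_ContainmentCharacter.
; CanInteract traces on the Visibility channel from the player camera along its forward vector up to InteractionDistance, with debug drawing.
; Despite its name, it also sends the Interact message to the hit actor and prints its name, then returns the hit result and actor.
; The event graph is empty, so the check runs only when called externally.
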(event `self.ReceiveTick`
  (params (DeltaSeconds :type "Float (single-precision)")))

(fn `CanInteract`
  (returns (CanInteract :type Boolean) (ActorInteracted :type "Actor Object Reference"))
  (locals (CameraStart :type "Vector Structure" :default (0.0 0.0 0.0)) (CameraEnd :type "Vector Structure"))
  (bind _asbp_containment_character (cast `/Game/Blueprints/BP_ContainmentCharacter` (`self.GetOwner`))
    (:`then`
      (bind _playercamera (`/Game/Blueprints/BP_ContainmentCharacter.PlayerCamera` _asbp_containment_character))
      (bind _output_get (set `local.CameraStart` (`SceneComponent.K2_GetComponentLocation` _playercamera)))
      (set `local.CameraEnd` (+ (* (`self.InteractionDistance`) (`SceneComponent.GetForwardVector` _playercamera)) _output_get))
      (bind (_outhit _returnvalue) (`KismetSystemLibrary.LineTraceSingle` :`Start` (`local.CameraStart`) :`End` (`local.CameraEnd`) :`TraceChannel` "TraceTypeQuery1" :`DrawDebugType` "ForDuration"))
      (if _returnvalue
        (bind (_bblockinghit _binitialoverlap _time _distance _location _impactpoint _normal _impactnormal _physmat _hitactor) (`GameplayStatics.BreakHitResult` _outhit))
        (`KismetSystemLibrary.PrintString` (`KismetStringLibrary.Concat_StrStr` "Interaction avec " (`KismetSystemLibrary.GetDisplayName` _hitactor)))
        (message `/Game/Blueprints/Interfaces/BPI_Interactable.Interact` _hitactor))
      (return _returnvalue _hitactor))
    (:`CastFailed`
      (return false _asbp_containment_character))))