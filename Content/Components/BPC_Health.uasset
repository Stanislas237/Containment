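; Health component that tracks an owner's current and maximum health and its death state.
; Health starts at maximum on BeginPlay; TakeDamage clamps the result, while SetHealth rejects out-of-range values.
; Changes fire an OnHealthChanged dispatcher, and reaching zero calls Die once, which sets IsDead and fires OnDeath.
; Getters expose raw and normalized health, and French debug messages are printed on screen.
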(event `self.ReceiveBeginPlay`
  (set `self.CurrentHealth` (`self.MaxHealth`)))

(fn `Die`
  (set `self.IsDead` true)
  (`KismetSystemLibrary.PrintString` "Vous êtes mort !" true true (struct :`R` 1.0 :`G` 0.030358 :`B` 0.046116 :`A` 1.0) 5.0)
  (`self.OnDeath`))

(fn `GetCurrentHealth`
  (returns (CurrentHealth :type "Float (double-precision)"))
  (return (`self.CurrentHealth`)))

(fn `GetCurrentHealthPercentage`
  (returns (CurrentHealthPercentage :type "Float (double-precision)"))
  (return (`KismetMathLibrary.FClamp` (/ (`self.CurrentHealth`) (`self.MaxHealth`)))))

(fn `SetHealth`
  (params (NewHealth :type "Float (double-precision)"))
  (locals (inNewHealth :type "Float (double-precision)") (PreviousHealth :type "Float (double-precision)"))
  (set `local.inNewHealth` NewHealth)
  (if (and (>= NewHealth 0.0) (<= NewHealth (`self.MaxHealth`)))
    (set `local.PreviousHealth` (`self.CurrentHealth`))
    (bind _output_get (set `self.CurrentHealth` (`local.inNewHealth`)))
    (`self.OnHealthChanged` (`local.PreviousHealth`) _output_get)
    (if (and (<= (`self.CurrentHealth`) 0.0) (not (`self.IsDead`)))
      (`self.Die`))
    (else
      (`KismetSystemLibrary.PrintString` (`KismetStringLibrary.Concat_StrStr` "Le paramètre passé à SetHealth (" (`KismetStringLibrary.Conv_DoubleToString` (`local.inNewHealth`)) ") doit être compris entre 0 et " (`KismetStringLibrary.Conv_DoubleToString` (`self.MaxHealth`))) true true (struct :`R` 1.0 :`G` 0.030358 :`B` 0.046116 :`A` 1.0) 5.0))))

(fn `TakeDamage`
  (params (Damages :type "Float (double-precision)"))
  (locals (fDamages :type "Float (double-precision)") (PreviousHealth :type "Float (double-precision)" :default 0.0))
  (set `local.fDamages` Damages)
  (set `local.PreviousHealth` (`self.CurrentHealth`))
  (bind _output_get (set `self.CurrentHealth` (`KismetMathLibrary.FClamp` (- (`self.CurrentHealth`) (`local.fDamages`)) 0.0 (`self.MaxHealth`))))
  (if (not (== (`self.CurrentHealth`) (`local.PreviousHealth`)))
    (`self.OnHealthChanged` (`local.PreviousHealth`) (`self.CurrentHealth`)))
  (if (and (<= _output_get 0.0) (not (`self.IsDead`)))
    (`self.Die`)
    (else
      (`KismetSystemLibrary.PrintString` (`KismetStringLibrary.Concat_StrStr` "Encaissé " (`KismetStringLibrary.Conv_DoubleToString` (`local.fDamages`)) " Il lui reste " (`KismetStringLibrary.Conv_DoubleToString` (`self.CurrentHealth`)) " PV sur " (`KismetStringLibrary.Conv_DoubleToString` (`self.MaxHealth`))) true true (struct :`R` 1.0 :`G` 0.030358 :`B` 0.753044 :`A` 1.0) 5.0))))