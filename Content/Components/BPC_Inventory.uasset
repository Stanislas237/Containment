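; Inventory component that adds items by ID and keeps each ID only once.
; AddItem rejects duplicates, then looks the ID up as a row name in the ItemsTable data table.
; A found row stores the ID, prints the item's display name in green and fires OnInventoryChanged with the new item count.
; Duplicates and missing rows only print a message.
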(fn `AddItem`
  (params (ItemID :type Name))
  (locals (nItemID :type Name))
  (set `local.nItemID` ItemID)
  (if (`KismetArrayLibrary.Array_Contains` (`self.Inventory`) (`local.nItemID`))
    (`KismetSystemLibrary.PrintString` "Already in inventory" true true (struct :`R` 1.0 :`G` 0.4799 :`B` 0.625203 :`A` 1.0) 20.0)
    (else
      (bind _returnvalue (`|GetDataTableRow` (`self.ItemsTable`) (`local.nItemID`))
        (:`then`
          (`KismetArrayLibrary.Array_Add` (`self.Inventory`) (`local.nItemID`))
          (`KismetSystemLibrary.PrintText` (`.DisplayName_6_94188EA0423F64C27A5255B97C272F67` (break `/Game/Data/ST_ItemData` _returnvalue)) true true (struct :`R` 0.067407 :`G` 1.0 :`B` 0.200069 :`A` 1.0) 20.0)
          (`self.OnInventoryChanged` (`KismetArrayLibrary.Array_Length` (`self.Inventory`))))
        (:`RowNotFound`
          (`KismetSystemLibrary.PrintString` "Row Not Found" true true (struct :`R` 1.0 :`G` 0.030358 :`B` 0.046116 :`A` 1.0) 20.0))))))